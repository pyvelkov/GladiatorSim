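; Peasant_Man_BP is a friendly male peasant AI pawn that moves around the world on BeginPlay according to its AIState.
; Roam sends it to a random navigable point within a radius of its location, then waits and repeats after each successful move.
; Walk sends it once to the Target1 actor, and a failed roam move ends the loop since only success is handled.
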(event `self.ReceiveBeginPlay`
  (switch `/Game/AI/friendly/Peasant/Man/Peasant_Man_Enum` (`self.AI state`)
    (:`NewEnumerator1`
      (`self.RoamTo`))
    (:`NewEnumerator0`
      (`self.WalkTo`))))

(event `WalkTo`
  (`|AIMoveTo` self (0.0 0.0 0.0) (`self.Target_1`)))

(event `RoamTo`
  (`|AIMoveTo` self (`NavigationSystemV1.K2_GetRandomLocationInNavigableRadius` (`self.K2_GetActorLocation`) 500.0 null null) null
    (:`OnSuccess`
      (`KismetSystemLibrary.Delay` 5.0)
      (`self.RoamTo`))))

(fn `UserConstructionScript`)