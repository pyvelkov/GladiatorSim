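; Dark_Female_BP is a friendly female AI pawn that walks a looping route between four target actors.
; BeginPlay leads into WalkTo, which chains AIMoveTo calls on success, pausing after the first and third targets.
; The last move continues from its immediate exec pin, so WalkTo restarts after a fixed delay without waiting for arrival at Target4.
; Failed moves are not handled.
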(event `self.ReceiveBeginPlay`
  (switch `/Game/AI/friendly/DarkChars/Woman/Dark_Female_Enum` (`self.AI State`)
    (:`NewEnumerator0`
      (`self.WalkTo`))))

(event `WalkTo`
  (`|AIMoveTo` self (0.0 0.0 0.0) (`self.Target_1`)
    (:`OnSuccess`
      (`KismetSystemLibrary.Delay` 3.0)
      (`|AIMoveTo` self (0.0 0.0 0.0) (`self.Target_2`)
        (:`OnSuccess`
          (`|AIMoveTo` self (0.0 0.0 0.0) (`self.target_3`)
            (:`OnSuccess`
              (`KismetSystemLibrary.Delay` 3.0)
              (`|AIMoveTo` self (0.0 0.0 0.0) (`self.target_4`)
                (:`then`
                  (`KismetSystemLibrary.Delay` 3.0)
                  (`self.WalkTo`))))))))))

(fn `UserConstructionScript`)