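; SpellCaster_BP is a spellcasting enemy that attacks the player with fireballs and can be killed by sword hits.
; When pawn sensing sees the player, it turns to face them and launches a FireBall_BP by impulse with a casting montage, gated by a cooldown.
; Sword overlaps during the player's slash reduce health, with brief invulnerability between hits.
; At zero health it stops AI logic, plays a death animation and destroys itself after a delay.
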(event `self.CapsuleComponent.OnComponentBeginOverlap`
  (params (OverlappedComponent :type "PrimitiveComponent Object Reference") (OtherActor :type "Actor Object Reference") (OtherComp :type "PrimitiveComponent Object Reference") (OtherBodyIndex :type Integer) (bFromSweep :type Boolean) (SweepResult :type "HitResult Structure (by ref)"))
  ;[1 1 1] health
  (cast `/Game/BluePrint_Character/sword/Weapon_Sword` OtherActor)
  (bind _ascharacter_bpnew (cast `/Game/BluePrint_Character/Character_BPnew` (`GameplayStatics.GetPlayerCharacter` 0)))
  (if (`/Game/BluePrint_Character/Character_BPnew.SlashSword` _ascharacter_bpnew)
    (if (`self.canBeHitWithMelee`)
      (`KismetSystemLibrary.PrintString` "Hello")
      (bind _output_get (set `self.Health` (- (`self.Health`) 1.0)))
      (if (<= _output_get 0.0)
        (`BrainComponent.StopLogic` (`AIController.BrainComponent` (`AIBlueprintHelperLibrary.GetAIController` self)) "")
        (`self.Death`)
        (`KismetSystemLibrary.Delay` 3.68)
        (`self.K2_DestroyActor`)
        (set `self.canBeHitWithMelee` false)
        (else
          (set `self.canBeHitWithMelee` false)
          (`KismetSystemLibrary.Delay` 2.0)
          (set `self.canBeHitWithMelee` true))))))

(event `self.PawnSensing.OnSeePawn`
  (params (Pawn :type "Pawn Object Reference"))
  ;[1 1 1] Ranged Attack
  (bind _ascharacter_bpnew (cast `/Game/BluePrint_Character/Character_BPnew` Pawn))
  (`|ExecutionSequence`
    (:`then_0`
      (`self.K2_SetActorRotation` (`KismetMathLibrary.FindLookAtRotation` (`self.K2_GetActorLocation`) (`self.K2_GetActorLocation` _ascharacter_bpnew))))
    (:`then_1`
      (if (`self.spawnProjectile`)
        (bind _returnvalue (`|SpawnActorFromClass` "/Game/AI/enemy2/fireball/fireBall_BP.fireBall_BP_C" (`SceneComponent.K2_GetComponentToWorld` (`self.projectile`)) "Undefined" "OverrideRootScale" null null))
        (`CharacterMovementComponent.DisableMovement` (`self.CharacterMovement`))
        (`MovementComponent.StopMovementImmediately` (`self.CharacterMovement`))
        (`self.PlayAnimMontage` "/Game/AI/enemy2/animations/Casting_Spell_Montage.Casting_Spell_Montage")
        (`CharacterMovementComponent.SetMovementMode` (`self.CharacterMovement`) "MOVE_Walking" 0)
        (`PrimitiveComponent.AddImpulse` (`/Game/AI/enemy2/fireball/fireBall_BP.Bullet` _returnvalue) (* (`SceneComponent.GetForwardVector` (`self.CapsuleComponent`)) (`KismetMathLibrary.FTrunc` (`self.projectileForce`))) "None" true)
        (set `self.spawnProjectile` false)
        (`KismetSystemLibrary.Delay` 1.3)
        (set `self.spawnProjectile` true)))))

(fn `Death`
  (if (<= (`self.Health`) 0.0)
    (`CharacterMovementComponent.DisableMovement` (`self.CharacterMovement`))
    (`MovementComponent.StopMovementImmediately` (`self.CharacterMovement`))
    (`SkeletalMeshComponent.PlayAnimation` (`self.Mesh`) "/Game/AI/enemy2/animations/Standing_React_Death_Forward.Standing_React_Death_Forward" false)))

(fn `UserConstructionScript`)